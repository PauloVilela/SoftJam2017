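; Base-looking projectile Blueprint that deals damage to either characters or enemies on contact.
; Its Collision overlap uses the IHurtCharater flag to pick the "Character" or "Enemy" actor tag, then applies Damage to a matching actor and destroys itself.
; BeginPlay starts a DeathTime delay with nothing wired after it, so only a matching hit destroys the projectile in this graph.
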(event OnComponentBeginOverlap(Collision)
  (params (OverlappedComponent :type Primitive%20Component%20Object%20Reference) (OtherActor :type Actor%20Object%20Reference) (OtherComp :type Primitive%20Component%20Object%20Reference) (OtherBodyIndex :type Integer) (bFromSweep :type Boolean) (SweepResult :type Hit%20Result%20Structure%20%28by%20ref%29))
  ;[1 1 1] On hit
  (if (Variables|Default|GetIHurtCharater)
    (if (Actor|ActorHasTag OtherActor "Character")
      (Game|Damage|ApplyDamage OtherActor (Variables|Default|GetDamage) 0 0)
      (Actor|DestroyActor))
    (elif (Actor|ActorHasTag OtherActor "Enemy")
      (Game|Damage|ApplyDamage OtherActor (Variables|Default|GetDamage) 0 0)
      (Actor|DestroyActor))))

(event EventBeginPlay
  ;[1 1 1] Sudoku
  (Utilities|FlowControl|Delay (Variables|Default|GetDeathTime)))

(fn ConstructionScript)