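; Primary bullet projectile that damages enemies and feeds mana back to the character who fired it.
; On overlap with an EnemyBase_CBP it applies its Damage, then adds the same amount as mana to the Base_CBP instigator.
; It destroys itself only after both casts succeed, so other overlaps, or a hit without a Base_CBP instigator, leave it alive.
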(event EventBeginPlay
  (|CallParentFunction) ; This node is disabled and will not be called.\nDrag off pins to build functionality.
)

(event Collision|EventActorBeginOverlap
  (params (OtherActor :type Actor%20Object%20Reference))
  (bind _asenemy_base_cbp (Utilities|Casting|CastToEnemyBase_CBP OtherActor))
  (Game|Damage|ApplyDamage _asenemy_base_cbp (Variables|Default|GetDamage) 0 0)
  ;[1 1 1] Add mana to character
  (bind _asbase_cbp (Utilities|Casting|CastToBase_CBP (Variables|Default|GetInstigator)))
  (Default|AddMana _asbase_cbp (Variables|Default|GetDamage))
  (Actor|DestroyActor))

(event EventTick
  (params (DeltaSeconds :type Float%20%28single-precision%29)))

(fn ConstructionScript
  (|CallParentFunction))