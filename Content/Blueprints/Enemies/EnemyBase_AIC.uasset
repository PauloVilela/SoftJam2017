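; AI controller for enemy pawns that sends them toward the world origin shortly after spawn, then chases and fires on a player.
; ChasePlayer compares distance against a fixed threshold: when far, it moves to a random navigable point around the player; when near, it calls Fire on EnemyBase_CBP and faces the player.
; A DoOnce gate limits repeated move requests, resetting on move success or when firing.
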(event Custom|ChasePlayer
  (params (Player :type Actor%20Object%20Reference) (Pawn :type Character%20Object%20Reference))
  (bind _returnvalue (Transformation|GetActorLocation Player))
  ;[1 1 1] Overlap chase player
  (Math|Float|CompareFloat (Transformation|GetDistanceTo Pawn Player) 5.1e+02
    (:>
      (Utilities|FlowControl|DoOnce false :!label _label
        (:Completed
          (AI|AIMoveTo Pawn (.RandomLocation (Class|NavigationSystem|GetRandomPointinNavigableRadius _returnvalue 5e+02)) 0 0.0 false
            (:OnSuccess
              (AI|SetFocalPoint _returnvalue)
              (goto _label Reset))))))
    (:==
      (goto _label))
    (:<
      ;[1 1 1] Fire
      (bind _asenemy_base_cbp (Utilities|Casting|CastToEnemyBase_CBP Pawn))
      (Default|Fire _asenemy_base_cbp)
      (CallFunction|ResetDoOnce)
      (AI|SetFocalPoint _returnvalue))))

(event Custom|ResetDoOnce
  ;[1 1 1] Overlap chase player
  (Utilities|FlowControl|DoOnce false) ; enters at Reset
)

(event EventBeginPlay
  ;[1 1 1] Go to the center of world
  (Utilities|FlowControl|Delay 0.1)
  (AI|AIMoveTo (Pawn|GetControlledPawn) "0, 0, 0" 0 0.0 false))

(fn ConstructionScript)