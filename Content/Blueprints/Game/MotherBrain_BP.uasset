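; MotherBrain is a wave manager that controls the level's EnemySpawner actors.
; On BeginPlay it gives every spawner a reference to itself and activates one at random.
; AddEnemy counts spawns and deactivates all spawners once the wave cap is reached.
; SomeOneDied checks for an empty AllEnemies list, then waits briefly, raises the cap, resets the count and activates a random spawner.
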(event Custom|AddEnemy
  (Variables|Default|SetSpawnEnemies (+ (Variables|Default|GetSpawnEnemies) 1))
  (if (<= (Variables|Default|GetMaxSpawnEnemies) (Variables|Default|GetSpawnEnemies))
    (for _array_element (Variables|Default|GetAllSpawnPoint)
      (Variables|/Game/Blueprints/Game/EnemySpawner.EnemySpawner_C|SetIsActive _array_element false))))

(event Custom|SomeOneDied
  (bind _allspawnpoint (Variables|Default|GetAllSpawnPoint))
  (if (<= (Utilities|Array|Length (Variables|Default|GetAllEnemies)) 0)
    (Utilities|FlowControl|Delay 2.0)
    (Variables|Default|SetMaxSpawnEnemies (+ (Variables|Default|GetMaxSpawnEnemies) 1))
    (Variables|Default|SetSpawnEnemies 0)
    (Variables|/Game/Blueprints/Game/EnemySpawner.EnemySpawner_C|SetIsActive (Utilities|Array|Get(acopy) _allspawnpoint (Math|Random|RandomInteger (Utilities|Array|Length _allspawnpoint))) true)))

(event EventBeginPlay
  (Utilities|FlowControl|Sequence
    (:then_0
      (bind _outactors (Actor|GetAllActorsOfClass "/Game/Blueprints/Game/EnemySpawner.EnemySpawner_C"))
      (bind _output_get (Variables|Default|SetAllSpawnPoint _outactors))
      (for _array_element _output_get
        (Variables|/Game/Blueprints/Game/EnemySpawner.EnemySpawner_C|SetMyBrain _array_element self)))
    (:then_1
      (Variables|/Game/Blueprints/Game/EnemySpawner.EnemySpawner_C|SetIsActive (Utilities|Array|Get(acopy) (Variables|Default|GetAllSpawnPoint) (Math|Random|RandomInteger (Utilities|Array|Length (Variables|Default|GetAllSpawnPoint)))) true))))

(fn ConstructionScript)