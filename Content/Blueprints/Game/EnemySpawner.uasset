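; Spawner actor that creates EnemyBase_CBP enemies at its own transform while IsActive is set.
; A random Delay on Tick acts as a repeating timer, spacing spawn attempts a few seconds apart, and spawns are skipped if colliding.
; Each enemy receives MyBrain as its MyMotherBrain, and the spawner adds it to the brain's AllEnemies list and calls AddEnemy.
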(event EventTick
  (params (DeltaSeconds :type Float%20%28single-precision%29))
  (bind _mybrain (Variables|Default|GetMyBrain))
  (Utilities|FlowControl|Delay (Math|Random|RandomFloatinRange 1.0 3.0))
  (if (Variables|Default|GetIsActive)
    (bind _returnvalue (Game|SpawnActorfromClass "/Game/Blueprints/Enemies/EnemyBase_CBP.EnemyBase_CBP_C" (Transformation|GetActorTransform) "DontSpawnIfColliding" 0 0))
    (Variables|/Game/Blueprints/Enemies/EnemyBase_CBP.EnemyBase_CBP_C|SetMyMotherBrain _returnvalue _mybrain)
    (Utilities|Array|Add (Variables|/Game/Blueprints/Game/MotherBrain_BP.MotherBrain_BP_C|GetAllEnemies _mybrain) _returnvalue)
    (Default|AddEnemy _mybrain)))

(fn ConstructionScript)