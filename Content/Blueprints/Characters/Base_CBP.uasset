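; Base twin-stick character that toggles between attack and defence modes, darkening its material colour for attack.
; Attack mode fires rate-limited shots or a held big shot, which locks movement while a timeline grows the projectile on the character.
; Defence mode spawns an attached shield while primary is held, and secondary dashes along velocity.
; Tick faces the character along the turn axes, and damage reduces health, destroying the actor at zero or below.
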(event Game|Damage|EventAnyDamage
  (params (Damage :type Float%20%28single-precision%29) (DamageType :type Damage%20Type%20Object%20Reference) (InstigatedBy :type Controller%20Object%20Reference) (DamageCauser :type Actor%20Object%20Reference))
  ;[1 1 1] health system
  (bind _output_get (Variables|Default|SetPlayerHealth (- (Variables|Default|GetPlayerHealth) Damage)))
  (Math|Float|CompareFloat _output_get 0.0
    (:==
      _)
    (:<
      _))
  (Actor|DestroyActor))

(event EventTick
  (params (DeltaSeconds :type Float%20%28single-precision%29))
  (bind _returnvalue (Input|AxisValues|GetTurnForward))
  (bind _returnvalue_2 (Input|AxisValues|GetTurnRight))
  (bind _returnvalue_3 (Math|Vector|MakeVector _returnvalue _returnvalue_2 0.0))
  (bind _returnvalue_4 (Math|Vector|RotateVector _returnvalue_3 "0,90.000000, 0"))
  ;[1 1 1] Input
  (if (> (Math|Vector|VectorLength _returnvalue_4) 0.0)
    (Transformation|SetActorRotation (Math|Rotator|MakeRotfromX _returnvalue_4))))

(event Input|ActionEvents|InputActionSecondaryAction
  (params (Key :type Key%20Structure))
  (bind _returnvalue (Transformation|GetActorRotation))
  (bind _returnvalue_2 (Transformation|GetActorLocation))
  (bind _firebigshot (Variables|Default|GetFireBigShot))
  ;[1 1 1] Input
  (:Pressed
    (if (Variables|Default|GetIsInAttackingMode)
      (Variables|Default|SetIsFiringBigShot true)
      (bind _returnvalue_3 (Game|SpawnActorfromClass "/Game/Blueprints/Weapons/Projectiles/DefaultProjectile_BP.DefaultProjectile_BP_C" (Math|Transform|MakeTransform _returnvalue_2 _returnvalue "1,1,1") "AlwaysSpawn" 0 0))
      (Variables|/Game/Blueprints/Weapons/Projectiles/DefaultProjectile_BP.DefaultProjectile_BP_C|SetIHurtCharater _returnvalue_3 false)
      (Timeline|FireBigShot PlayFromStart
        (:Update
          (Transformation|SetActorTransform _returnvalue_3 (Math|Transform|MakeTransform _returnvalue_2 _returnvalue (* "1.000000,1.000000,1.000000" (+ (/ (Components|Timeline|GetPlaybackPosition _firebigshot) (Components|Timeline|GetTimelineLength _firebigshot)) 1.0)))))
        (:Finished
          (Variables|Default|SetIsFiringBigShot false)))
      (else
        ;;[1 1 1] Dashing like a mad man
        (Character|LaunchCharacter (* (Math|Vector|Normalize (Transformation|GetVelocity)) 1e+03) false false))))
  (:Released
    (Variables|Default|SetIsFiringBigShot false)
    (Timeline|FireBigShot Stop)))

(event Input|ActionEvents|InputActionPrimaryAction
  (params (Key :type Key%20Structure))
  ;[1 1 1] Input
  (:Pressed
    (if (not (Variables|Default|GetIsInAttackingMode))
      (CallFunction|ShieldMe)))
  (:Released
    (if (!= (Variables|Default|GetMyShield) 0)
      (Actor|DestroyActor (Variables|Default|GetMyShield))
      (Variables|Default|SetMyShield 0))))

(event Input|ActionEvents|InputActionSwitchMode
  (params (Key :type Key%20Structure))
  (bind _firebigshot (Variables|Default|GetFireBigShot))
  ;[1 1 1] Input
  (:Pressed
    (Utilities|FlowControl|FlipFlop
      (:A
        (Variables|Default|SetIsInAttackingMode true)
        (CallFunction|ChangeColor)
        ;;[1 1 1] Remove Shield when going to AMode
        (if (!= (Variables|Default|GetMyShield) 0)
          (Actor|DestroyActor (Variables|Default|GetMyShield))
          (Variables|Default|SetMyShield 0)))
      (:B
        (Variables|Default|SetIsInAttackingMode false)
        (CallFunction|ChangeColor)
        (Timeline|FireBigShot Stop
          (:Update
            (Transformation|SetActorTransform (stale Input|ActionEvents|InputActionSecondaryAction _returnvalue_3) (Math|Transform|MakeTransform (Transformation|GetActorLocation) (Transformation|GetActorRotation) (* "1.000000,1.000000,1.000000" (+ (/ (Components|Timeline|GetPlaybackPosition _firebigshot) (Components|Timeline|GetTimelineLength _firebigshot)) 1.0)))))
          (:Finished
            (Variables|Default|SetIsFiringBigShot false)))))))

(event Input|AxisEvents|InputAxisMoveForward
  (params (AxisValue :type Float%20%28single-precision%29))
  ;[1 1 1] Input
  (if (not (Variables|Default|GetIsFiringBigShot))
    (Pawn|Input|AddMovementInput "1.000000, 0, 0" AxisValue false)))

(event Input|AxisEvents|InputAxisMoveRight
  (params (AxisValue :type Float%20%28single-precision%29))
  ;[1 1 1] Input
  (if (not (Variables|Default|GetIsFiringBigShot))
    (Pawn|Input|AddMovementInput "0,1.000000,0.000000" AxisValue false)))

(event Input|AxisEvents|InputAxisPrimaryAction
  (params (AxisValue :type Float%20%28single-precision%29))
  ;[1 1 1] Input
  (if (and (!= AxisValue 0.0) (Variables|Default|GetIsInAttackingMode))
    (if (not (Variables|Default|GetIsFiringBigShot))
      (CallFunction|FireShot)
      (Utilities|FlowControl|Delay (Variables|Default|GetFiringRate))
      (Variables|Default|SetCanFire true))))

(fn ConstructionScript
  (bind _returnvalue (Rendering|Material|CreateDynamicMaterialInstance (Variables|Character|GetMesh) 0 0 :!class /Script/Engine.PrimitiveComponent))
  (bind _output_get (Variables|Default|SetMyDynamicMAT _returnvalue))
  (bind _returnvalue_2 (Rendering|Material|GetVectorParameterValue _output_get "Colour" :!class /Script/Engine.MaterialInstanceDynamic))
  (bind _output_get_2 (Variables|Default|SetDefenseColour _returnvalue_2))
  (Variables|Default|SetAttackColour (* _output_get_2 0.5))
  (CallFunction|ChangeColor))

(fn FireShot
  (bind _returnvalue (Transformation|GetActorRotation))
  (if (Variables|Default|GetCanFire)
    (bind _returnvalue_2 (Game|SpawnActorfromClass "/Game/Blueprints/Weapons/Projectiles/DefaultProjectile_BP.DefaultProjectile_BP_C" (Math|Transform|MakeTransform (+ (Transformation|GetActorLocation) (* (Math|Vector|GetForwardVector _returnvalue) 1e+02)) _returnvalue "1,1,1") "AlwaysSpawn" 0 0))
    (Variables|/Game/Blueprints/Weapons/Projectiles/DefaultProjectile_BP.DefaultProjectile_BP_C|SetIHurtCharater _returnvalue_2 false)
    (Variables|Default|SetCanFire false)))

(fn ShieldMe
  (bind _returnvalue (Transformation|GetActorRotation))
  (bind _returnvalue_2 (Game|SpawnActorfromClass "/Game/Blueprints/Weapons/DefaultShield_BP.DefaultShield_BP_C" (Math|Transform|MakeTransform (+ (Transformation|GetActorLocation) (* (Math|Vector|GetForwardVector _returnvalue) (Variables|Default|GetShieldRadius))) _returnvalue "1,1,1") "AlwaysSpawn" 0 0))
  (Transformation|AttachActorToActor _returnvalue_2 self "None" "KeepWorld" "KeepWorld" "KeepWorld" true)
  (Variables|Default|SetMyShield _returnvalue_2))

(fn ChangeColor
  (if (Variables|Default|GetIsInAttackingMode)
    (Rendering|Material|SetVectorParameterValue (Variables|Default|GetMyDynamicMAT) "Colour" (Variables|Default|GetAttackColour) :!class /Script/Engine.MaterialInstanceDynamic)
    (else
      (Rendering|Material|SetVectorParameterValue (Variables|Default|GetMyDynamicMAT) "Colour" (Variables|Default|GetDefenseColour) :!class /Script/Engine.MaterialInstanceDynamic))))